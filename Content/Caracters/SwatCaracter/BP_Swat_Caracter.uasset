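; Player SWAT character with Enhanced Input movement, walk/run, aiming and AK-47 fire.
; BeginPlay attaches a spawned weapon and creates HUD and crosshair widgets; Tick updates left-hand grip location, ammo text and CanShoot.
; Aiming switches to controller-yaw rotation, shows the crosshair and slides the camera via timeline.
; DoOnce-gated shots need aiming, spend ammo and trace camera-to-target, then muzzle-to-target with debug drawing only; a debug key tests health.
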(event Input|EnhancedActionEvents|EnhancedInputActionIA_Move
  (params (ActionValue :type Vector%202D%20Structure) (ElapsedSeconds :type Float%20%28double-precision%29) (TriggeredSeconds :type Float%20%28double-precision%29) (InputAction :type Input%20Action%20Object%20Reference :default "/Game/Data/Inputs/IA_Move.IA_Move"))
  (bind _returnvalue (Pawn|GetControlRotation :!class /Script/Engine.Pawn))
  ;[0.15 0.05485 0.05091 0.5] Add movment settings
  (Pawn|Input|AddMovementInput (Math|Vector|GetRightVector (Math|Rotator|MakeRotator (.roll _returnvalue) 0.0 (.yaw _returnvalue))) (.x ActionValue) false)
  (Pawn|Input|AddMovementInput (Math|Vector|GetForwardVector (Math|Rotator|MakeRotator 0.0 0.0 (.yaw (Pawn|GetControlRotation :!class /Script/Engine.Pawn)))) (.y ActionValue) false))

(event Input|EnhancedActionEvents|EnhancedInputActionIA_Look
  (params (ActionValue :type Vector%202D%20Structure) (ElapsedSeconds :type Float%20%28double-precision%29) (TriggeredSeconds :type Float%20%28double-precision%29) (InputAction :type Input%20Action%20Object%20Reference :default "/Game/Data/Inputs/IA_Look.IA_Look"))
  ;[0.02846 0.03951 0.15 0.5] Mause controll attachment
  (Pawn|Input|AddControllerYawInput (.x ActionValue))
  (Pawn|Input|AddControllerPitchInput (.y ActionValue)))

(event Input|EnhancedActionEvents|EnhancedInputActionIA_RunWalk
  (params (ActionValue :type Boolean) (ElapsedSeconds :type Float%20%28double-precision%29) (TriggeredSeconds :type Float%20%28double-precision%29) (InputAction :type Input%20Action%20Object%20Reference :default "/Game/Data/Inputs/IA_RunWalk.IA_RunWalk"))
  (bind _charactermovement (Variables|Character|GetCharacterMovement))
  ;[0.15 0.04802 0.01434 0.5] Run/walk key Attachment
  (:Triggered
    (Variables|/Script/Engine.CharacterMovementComponent|SetMaxWalkSpeed _charactermovement 4e+02))
  (:Canceled
    (Variables|/Script/Engine.CharacterMovementComponent|SetMaxWalkSpeed _charactermovement 2e+02 :!label _label))
  (:Completed
    (goto _label)))

(event Input|EnhancedActionEvents|EnhancedInputActionIA_Aiming
  (params (ActionValue :type Boolean) (ElapsedSeconds :type Float%20%28double-precision%29) (TriggeredSeconds :type Float%20%28double-precision%29) (InputAction :type Input%20Action%20Object%20Reference :default "/Game/Data/Inputs/IA_Aiming.IA_Aiming"))
  (bind _camera (Variables|Default|GetCamera))
  (bind _charactermovement (Variables|Character|GetCharacterMovement))
  (bind _wbp_maincrosshair (Variables|Default|GetWBP_MainCrosshair))
  (bind _wbp_maincrosshair_2 (Variables|Default|GetWBP_MainCrosshair))
  (bind _relativelocation (Variables|/Script/Engine.SceneComponent|GetRelativeLocation _camera))
  (:Started
    (Variables|Default|SetbIsAimming true)
    (Variables|/Script/Engine.CharacterMovementComponent|SetbOrientRotationToMovement _charactermovement false)
    (Variables|Default|SetbUseControllerRotationYaw true)
    (UserInterface|Viewport|AddtoViewport _wbp_maincrosshair 0)
    (bind _newtrack_0 (Timeline|TL_Aim_Animation_Cam Play)
      (:Update
        (Transformation|SetRelativeLocation _camera (Math|Vector|MakeVector (Math|Float|Lerp 75.640621 1.5e+02 _newtrack_0) (.y _relativelocation) (.z _relativelocation)) false false)
        (Class|UserWidget|PlayAnimationForward _wbp_maincrosshair_2 (Variables|/Game/Caracters/Widgets/WBPCrossHair.WBPCrossHair_C|GetCrossSizeAiming _wbp_maincrosshair_2) 1.0 false))))
  (:Canceled
    (Variables|Default|SetbIsAimming false :!label _label)
    (Variables|/Script/Engine.CharacterMovementComponent|SetbOrientRotationToMovement _charactermovement true)
    (Variables|Default|SetbUseControllerRotationYaw false)
    (Widget|RemovefromParent _wbp_maincrosshair)
    (Timeline|TL_Aim_Animation_Cam Reverse))
  (:Completed
    (goto _label)))

(event Input|EnhancedActionEvents|EnhancedInputActionIA_Shoot
  (params (ActionValue :type Boolean) (ElapsedSeconds :type Float%20%28double-precision%29) (TriggeredSeconds :type Float%20%28double-precision%29) (InputAction :type Input%20Action%20Object%20Reference :default "/Game/Data/Inputs/IA_Shoot.IA_Shoot"))
  (:Triggered
    (Utilities|FlowControl|DoOnce false :!label _label
      (:Completed
        (if (Variables|Default|GetbIsAimming)
          (if (Variables|Default|GetbCanShoot)
            (Animation|Montage|PlayMontage (Variables|Character|GetMesh) "/Game/Caracters/Animations/Firing_Rifle_Montage.Firing_Rifle_Montage"
              (:then
                (Default|ShootLight (Variables|Default|GetBP_Weapon))
                (Audio|SpawnSound2D "/Game/Data/Sounds/AK_Sound_Wav.AK_Sound_Wav" 1.0 (Math|Float|Clamp(Float) (Math|Random|RandomFloat) 0.9 1.1) 0.0 0)
                (AddComponent|AddCameraShakeSourceComponent false (Transformation|GetRelativeTransform (Variables|Default|GetCamera)))
                (CallFunction|MunitionCounter)
                (CallFunction|LineTrace)
                (Utilities|FlowControl|Delay 0.1)
                (goto _label Reset)))
            (else
              (Audio|SpawnSound2D "/Game/Data/Sounds/EmptyAK.EmptyAK" 1.0 (Math|Float|Clamp(Float) (Math|Random|RandomFloat) 0.9 1.1) 0.0 0)))))))
  (:Canceled
    (Variables|Default|SetbCanShoot false)
    (Animation|StopAnimMontage "/Game/Caracters/Animations/Firing_Rifle_Montage.Firing_Rifle_Montage")))

(event EventBeginPlay
  (Utilities|FlowControl|Sequence
    (:then_0
      ;[0.0539 0.15 0.01558 0.5] Attachmente weapon to Character
      (bind _returnvalue (Game|SpawnActorfromClass "/Game/FPS_Weapon_Bundle/BP_Weapon.BP_Weapon_C" (Transformation|GetSocketTransform (Variables|Character|GetMesh) "WeaponSocket" "RTS_World") "Undefined" "MultiplyWithRoot" 0 0))
      (bind _output_get (Variables|Default|SetBP_Weapon _returnvalue))
      (Transformation|AttachComponentToComponent _output_get (Variables|Character|GetMesh) "WeaponSocket" "SnapToTarget" "SnapToTarget" "SnapToTarget" true))
    (:then_1
      ;[0.1447 0.02699 0.15 0.5] MoveKeysAutoConnection
      (bind _asplayer_controller (Utilities|Casting|CastToPlayerController (Pawn|GetController)))
      (Input|AddMappingContext (PlayerController|LocalPlayerSubsystems|GetEnhancedInputLocalPlayerSubsystem _asplayer_controller) "/Game/Data/Inputs/IMC_Default_Buttons.IMC_Default_Buttons" 0 "(bIgnoreAllPressedKeysUntilRelease=True,bForceImmediately=False,bNotifyUserSettings=False)"))
    (:then_2
      (bind _returnvalue_2 (UserInterface|CreateWidget "/Game/Caracters/Widgets/WBPCrossHair.WBPCrossHair_C"))
      (Variables|Default|SetWBP_MainCrosshair _returnvalue_2)
      (bind _returnvalue_3 (UserInterface|CreateWidget "/Game/Caracters/Widgets/WBP_MainWidget.WBP_MainWidget_C"))
      (bind _output_get_2 (Variables|Default|SetWBP_MainWidget _returnvalue_3))
      (UserInterface|Viewport|AddtoViewport _output_get_2 0))))

(event EventTick
  (params (DeltaSeconds :type Float%20%28single-precision%29))
  (Variables|Default|SetAK47WeaponLeftHandLocation (.location (Transformation|GetSocketTransform (Variables|/Game/FPS_Weapon_Bundle/BP_Weapon.BP_Weapon_C|GetWeaponSkeleton (Variables|Default|GetBP_Weapon)) "LeftHandPassition" "RTS_World")))
  (if (== (Variables|Default|GetMunition) 0)
    (Variables|Default|SetbCanShoot false)
    (else
      (Variables|Default|SetbCanShoot true)))
  (Rendering|Components|TextRender|SetText (Variables|/Game/Caracters/Widgets/WBP_MainWidget.WBP_MainWidget_C|GetWeaponCounter (Variables|Default|GetWBP_MainWidget)) (Utilities|Text|ToText(Integer) (Variables|Default|GetMunition))))

(event Input|KeyboardEvents|DebugKey1
  (params (Key :type Key%20Structure :default "None") (ActionValue :type Input%20Action%20Value%20Structure))
  (:Pressed
    (bind _health (Default|FuncHit (Variables|Default|GetAC_Health)))
    (Progress|SetPercent (Variables|/Game/Caracters/Widgets/WBP_MainWidget.WBP_MainWidget_C|GetPG_HealthBar (Variables|Default|GetWBP_MainWidget)) _health)))

(fn ConstructionScript)

(fn LineTrace
  (bind _returnvalue (Game|GetPlayerCameraManager 0))
  (bind _returnvalue_2 (Transformation|GetActorLocation _returnvalue))
  (bind _outhit (Collision|LineTraceByChannel _returnvalue_2 (+ _returnvalue_2 (* (Transformation|GetActorForwardVector _returnvalue) 5e+04)) "TraceTypeQuery1" false 0 "None"))
  (if (.bBlockingHit (Collision|BreakHitResult _outhit))
    (Collision|LineTraceByChannel (Transformation|GetWorldLocation (Variables|/Game/FPS_Weapon_Bundle/BP_Weapon.BP_Weapon_C|GetArrow (Variables|Default|GetBP_Weapon))) (.ImpactPoint (Collision|BreakHitResult _outhit)) "TraceTypeQuery1" false 0 "ForDuration")
    (else
      (Collision|LineTraceByChannel (Transformation|GetWorldLocation (Variables|/Game/FPS_Weapon_Bundle/BP_Weapon.BP_Weapon_C|GetArrow (Variables|Default|GetBP_Weapon))) (.TraceEnd (Collision|BreakHitResult _outhit)) "TraceTypeQuery1" false 0 "ForDuration"))))

(fn MunitionCounter
  (Variables|Default|SetMunition (Math|Integer|Clamp(Integer) (- (Variables|Default|GetMunition) 1) 0 30)))